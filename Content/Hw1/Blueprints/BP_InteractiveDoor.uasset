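; BP_InteractiveDoor is a hinged door that the first player character can open once while overlapping it, with no closing logic.
; BeginPlay stores the hinge's closed rotation and configures the Timeline's length from OpenDuration, with a small minimum.
; TryOpen validates the requester and door state, then plays the Timeline.
; Each update rotates the hinge's yaw linearly toward OpenAngle from playback progress, and finishing marks the door open.
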(event EventBeginPlay
  (Variables|Default|SetClosedRotation (Variables|/Script/Engine.SceneComponent|GetRelativeRotation (Variables|Default|GetHingePivot)))
  (Components|Timeline|SetTimelineLength (Variables|Default|GetTimeline) (select (> (Variables|Default|GetOpenDuration) (Math|Float|MakeLiteralFloat 0.01)) (Variables|Default|GetOpenDuration) (Math|Float|MakeLiteralFloat 0.01)))
  (Class|TimelineComponent|SetTimelineLengthMode (Variables|Default|GetTimeline) "TL_TimelineLength")
  (Timeline|Timeline Stop
    (:Update
      (CallFunction|UpdateDoorRotation))
    (:Finished
      (CallFunction|FinishOpening))))

(event Collision|EventActorBeginOverlap
  (params (OtherActor :type Actor%20Object%20Reference)))

(event EventTick
  (params (DeltaSeconds :type Float%20%28single-precision%29)))

(fn ConstructionScript)

(fn UpdateDoorRotation
  (bind _timeline (Variables|Default|GetTimeline))
  (Transformation|SetRelativeRotation (Variables|Default|GetHingePivot) (Math|Rotator|CombineRotators (Variables|Default|GetClosedRotation) (Math|Rotator|MakeRotator 0.0 0.0 (* (/ (Components|Timeline|GetPlaybackPosition _timeline) (Components|Timeline|GetTimelineLength _timeline)) (Variables|Default|GetOpenAngle)))) false true))

(fn FinishOpening
  (Variables|Default|SetbIsOpen true)
  (Variables|Default|SetbOpening false))

(fn TryOpen
  (params (RequestingPlayer :type Actor%20Object%20Reference))
  (if (and (and (not (Variables|Default|GetbIsOpen)) (not (Variables|Default|GetbOpening))) (and (== RequestingPlayer (Game|GetPlayerCharacter 0)) (Collision|IsOverlappingActor self RequestingPlayer :!class /Script/Engine.Actor)))
    (Variables|Default|SetbOpening true)
    (Components|Timeline|PlayfromStart (Variables|Default|GetTimeline))))